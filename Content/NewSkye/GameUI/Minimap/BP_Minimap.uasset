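; BP_Minimap is an actor that sets up the in-game minimap and supplies it with the player's position.
; On BeginPlay it creates the WBP_Minimap widget and adds it to the viewport.
; Each Tick it writes the controlled pawn's location into the MP_MInimap material parameter collection.
; It also sets the Player Yaw parameter to a constant zero, so pawn rotation is not passed through.
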(event EventBeginPlay
  (bind _returnvalue (UserInterface|CreateWidget "/Game/NewSkye/GameUI/Minimap/WBP_Minimap.WBP_Minimap_C"))
  (UserInterface|Viewport|AddtoViewport _returnvalue 0))

(event Collision|EventActorBeginOverlap
  (params (OtherActor :type Actor%20Object%20Reference)))

(event EventTick
  (params (DeltaSeconds :type Float%20%28single-precision%29))
  (Rendering|Material|SetVectorParameterValue "/Game/NewSkye/GameUI/Minimap/MP_MInimap.MP_MInimap" "Player Location" (Math|Conversions|ToLinearColor(Vector) (Transformation|GetActorLocation (Pawn|GetControlledPawn (Game|GetPlayerController 0)))) :!class /Script/Engine.KismetMaterialLibrary)
  (Rendering|Material|SetScalarParameterValue "/Game/NewSkye/GameUI/Minimap/MP_MInimap.MP_MInimap" "Player Yaw" 0.0 :!class /Script/Engine.KismetMaterialLibrary))

(fn ConstructionScript)