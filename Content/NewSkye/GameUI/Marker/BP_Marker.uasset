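; BP_Marker is an objective marker actor whose widget component displays the player's distance to it in meters.
; While MarkerHidden is true, Tick computes the rounded distance to the controlled pawn and pushes it to a lazily cached WBP_Marker.
; MarkerHidden also sets widget visibility directly, so true means shown despite the name.
; A Bp_Tank entering the Box sets it false, hiding the marker and stopping updates.
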(event OnComponentBeginOverlap(Box)
  (params (OverlappedComponent :type Primitive%20Component%20Object%20Reference) (OtherActor :type Actor%20Object%20Reference) (OtherComp :type Primitive%20Component%20Object%20Reference) (OtherBodyIndex :type Integer) (bFromSweep :type Boolean) (SweepResult :type Hit%20Result%20Structure%20%28by%20ref%29))
  (Utilities|Casting|CastToBp_Tank OtherActor)
  (CallFunction|ToggleObjectiveMarker false))

(event EventBeginPlay)

(event Collision|EventActorBeginOverlap
  (params (OtherActor :type Actor%20Object%20Reference)))

(event EventTick
  (params (DeltaSeconds :type Float%20%28single-precision%29))
  (if (Variables|Default|GetMarkerHidden)
    (CallFunction|UpdateDistance)))

(fn ConstructionScript
  (Rendering|SetVisibility (Variables|Default|GetWidget) (Variables|Default|GetMarkerHidden) false))

(fn UpdateDistance
  (Variables|Default|GetWBP%20Marker
    (:then
      _)
    (:else
      (bind _aswbp_marker (Utilities|Casting|CastToWBP_Marker (UserInterface|GetUserWidgetObject (Variables|Default|GetWidget))))
      (Variables|Default|SetWBP%20Marker _aswbp_marker)))
  (Default|UpdateText (Variables|Default|GetWBP%20Marker) (Utilities|String|Append (Utilities|String|ToString(Integer) (Math|Float|Round (/ (Math|Vector|VectorLength (- (Transformation|GetActorLocation) (Transformation|GetActorLocation (Pawn|GetControlledPawn (Game|GetPlayerController 0))))) 1e+02))) "m")))

(fn ToggleObjectiveMarker
  (params (MarkerHidden :type Boolean))
  (bind _output_get (Variables|Default|SetMarkerHidden MarkerHidden))
  (Rendering|SetVisibility (Variables|Default|GetWidget) _output_get false))