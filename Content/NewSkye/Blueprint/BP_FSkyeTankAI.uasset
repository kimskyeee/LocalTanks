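; AI tank pawn run by AIC_FSkyeTank that roams, aims at the player, fires shells and takes damage.
; AIMovement averages ground-sensor hits to align the hull to terrain while interpolating speed and rotation.
; Looping timers turn turret and gun toward the player or a blackboard random rotation, writing moving flags to the blackboard.
; BPCDamageSystem feeds a health bar widget, and Death requests a role-based respawn from BP_TankGameMode before destroying tank and controller.
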(event Custom|TurretRotOnly
  (bind _returnvalue (Utilities|Time|SetTimerbyFunctionName 0 "TurretRotateToTargetActor" 0.1 true))
  (Variables|Default|SetTurretHandle _returnvalue))

(event Custom|RandomRoam
  (AI|AIMoveTo self (.RandomLocation (AI|Navigation|GetRandomReachablePointinRadius (Transformation|GetActorLocation) 1.3e+04 0 0)) 0 5.0 false))

(event Custom|OnDeath)

(event Custom|SetRandRot
  (bind _returnvalue (Utilities|Time|SetTimerbyFunctionName 0 "DistanceCalculate" 0.1 true))
  (Variables|Default|SetRandomrotHandle _returnvalue))

(event Custom|Death
  (bind _asbp_tank_game_mode (Utilities|Casting|CastToBP_TankGameMode (Game|GetGameMode)))
  (Class|TankGameMode|RespawnTank _asbp_tank_game_mode (Variables|Default|GetRoleID))
  (Actor|DestroyActor (Pawn|GetController))
  (Actor|DestroyActor))

(event Custom|Block
  (params (CanBeParried :type Boolean))
  (Development|PrintString "Blocked"))

(event Custom|Attack
  (bind _bullethere (Variables|Default|GetBulletHere))
  (bind _returnvalue (Transformation|GetWorldLocation _bullethere))
  (bind _returnvalue_2 (Transformation|GetWorldRotation _bullethere))
  (Class|MyPawn|Fire _returnvalue _returnvalue_2)
  (Effects|SpawnEmitteratLocation "/Game/VigilanteContent/Vehicles/West_Tank_M1A1Abrams/FX/PS_MuzzleFire_01_M1A1Abrams.PS_MuzzleFire_01_M1A1Abrams" _returnvalue _returnvalue_2))

(event Custom|GunRot
  (bind _returnvalue (Utilities|Time|SetTimerbyFunctionName 0 "GunRotateToTargetActor" 0.1 true))
  (Variables|Default|SetGunHandle _returnvalue))

(event EventBeginPlay
  (bind _bpc_damagesystem (Variables|Default|GetBPC_DamageSystem))
  (bind _maxhealth (Variables|/Game/NewSkye/Blueprint/AI_DamageSystem/BPC_DamageSystem.BPC_DamageSystem_C|GetMaxHealth _bpc_damagesystem))
  (bind _asaic_fskye_tank (Utilities|Casting|CastToAIC_FSkyeTank (Pawn|GetController)))
  (AI|Components|Blackboard|SetValueasEnum (Variables|/Script/AIModule.AIController|GetBlackboard _asaic_fskye_tank) (Utilities|Name|MakeLiteralName "Role"))
  (bind _returnvalue (Actor|GetActorOfClass "/Game/BuildingDestruction/Tank/Bp_Tank.Bp_Tank_C"))
  (Variables|Default|SetPlayerD (Transformation|GetActorLocation _returnvalue))
  (bind _returnvalue_2 (Actor|GetActorOfClass "/Game/NewSkye/Blueprint/BP_Destination.BP_Destination_C"))
  (Variables|Default|SetDestiVec (Transformation|GetActorLocation _returnvalue_2))
  (Variables|Default|SetGround%20Sensing (Actor|GetComponentsByClass "/Game/NewSkye/Blueprint/BP_GroundSensing.BP_GroundSensing_C"))
  (Variables|/Game/NewSkye/Blueprint/AI_DamageSystem/BPC_DamageSystem.BPC_DamageSystem_C|SetHealth _bpc_damagesystem _maxhealth)
  (bind _returnvalue_3 (UserInterface|CreateWidget "/Game/NewSkye/PlayerUI/WBP_HealthBar.WBP_HealthBar_C"))
  (UserInterface|SetWidget (Variables|Default|GetHealthBar) _returnvalue_3)
  (Default|PercentUpdate _returnvalue_3 _maxhealth _maxhealth))

(event EventTick
  (params (DeltaSeconds :type Float%20%28single-precision%29)))

(fn ConstructionScript
  (bind _bpc_damagesystem (Variables|Default|GetBPC_DamageSystem))
  (EventDispatchers|BindEventtoOnDeath _bpc_damagesystem (EventDispatchers|CreateEvent :!event Custom|Death))
  (EventDispatchers|BindEventtoOnBlocked _bpc_damagesystem (EventDispatchers|CreateEvent :!event Custom|Block)))

(fn AIMovement
  (bind _returnvalue (Utilities|Time|GetWorldDeltaSeconds))
  (bind _returnvalue_2 (Utilities|Time|GetWorldDeltaSeconds))
  (Variables|Default|SetAverageNormal "0, 0, 0")
  (Variables|Default|SetAverageHeight 0.0)
  (Variables|Default|SetCountOnGround 0)
  (for _array_element (Variables|Default|GetGround%20Sensing)
    (Variables|Default|SetAverageNormal (+ (Variables|/Game/NewSkye/Blueprint/BP_GroundSensing.BP_GroundSensing_C|GetHitNormal _array_element) (Variables|Default|GetAverageNormal)))
    (Variables|Default|SetAverageHeight (+ (.z (Variables|/Game/NewSkye/Blueprint/BP_GroundSensing.BP_GroundSensing_C|GetHitLocation _array_element)) (Variables|Default|GetAverageHeight)))
    (if (Variables|/Game/NewSkye/Blueprint/BP_GroundSensing.BP_GroundSensing_C|GetbOnGround _array_element)
      (Math|Integer|IncrementInt (Variables|Default|GetCountOnGround))))
  (Variables|Default|SetAverageNormal (/ (Variables|Default|GetAverageNormal) (Variables|Default|GetCountOnGround)))
  (bind _output_get (Variables|Default|SetAverageHeight (/ (Variables|Default|GetAverageHeight) (Variables|Default|GetCountOnGround))))
  (Variables|Default|SetDeltaZ (- (+ _output_get (Variables|Default|GetHeightOffset)) (.z (Transformation|GetActorLocation))))
  (Utilities|FlowControl|Sequence
    (:then_1
      (Transformation|SetActorRotation (Math|Interpolation|RInterpTo (Transformation|GetActorRotation) (Math|Rotator|CombineRotators (Math|Rotator|MakeRotator 0.0 0.0 (* (Variables|Default|GetTargetTurnSpeed) _returnvalue_2)) (Math|Rotator|MakeRotfromZY (Variables|Default|GetAverageNormal) (Transformation|GetActorRightVector))) _returnvalue_2 3.0))
      (Transformation|AddActorWorldOffset (+ (* (Transformation|GetActorForwardVector) (Math|Interpolation|FInterpTo (Variables|Default|GetCurrent%20Forward%20Speed) (Variables|Default|GetTargetForwardSpeed) _returnvalue 3.0) _returnvalue) (* (Transformation|GetActorUpVector) (Variables|Default|GetDeltaZ))))
      (Variables|Default|SetCurrent%20Forward%20Speed (Math|Interpolation|FInterpTo (Variables|Default|GetCurrent%20Forward%20Speed) (Variables|Default|GetTargetForwardSpeed) _returnvalue 3.0)))))

(fn AIRotatetoTargetActor
  (Transformation|SetActorRotation (Math|Interpolation|RInterpTo (Transformation|GetActorRotation) (Math|Rotator|MakeRotator 0.0 0.0 (.yaw (Math|Rotator|FindLookatRotation (Transformation|GetActorLocation) (Transformation|GetActorLocation (Pawn|GetControlledPawn (Game|GetPlayerController 0)))))) (Utilities|Time|GetWorldDeltaSeconds) 3.0)))

(fn TurretRotatetoTargetActor
  (bind _returnvalue (Game|GetPlayerController 0))
  (bind _self self)
  (bind _box1 (Variables|Default|GetBox1))
  (bind _returnvalue_2 (Transformation|GetActorTransform _self))
  (bind _returnvalue_3 (Pawn|GetControlledPawn _returnvalue))
  (bind _relativerotation (Variables|/Script/Engine.SceneComponent|GetRelativeRotation _box1))
  (bind _returnvalue_4 (Transformation|GetActorLocation _returnvalue_3))
  (bind _returnvalue_5 (Math|Transform|InverseTransformLocation _returnvalue_2 _returnvalue_4))
  (bind _returnvalue_6 (Class|KismetMathLibrary|DegAtan2 (.y _returnvalue_5) (.x _returnvalue_5)))
  (bind _returnvalue_7 (Math|Rotator|NormalizeAxis _returnvalue_6))
  (bind _returnvalue_8 (- _returnvalue_7 (.yaw _relativerotation)))
  (bind _returnvalue_9 (Math|Rotator|NormalizeAxis _returnvalue_8))
  (bind _returnvalue_10 (Math|Float|Absolute(Float) _returnvalue_9))
  (bind _returnvalue_11 (<= _returnvalue_10 1.0))
  (bind _returnvalue_12 (not _returnvalue_11))
  (Transformation|SetRelativeRotation (Variables|Default|GetBox1) (Math|Rotator|MakeRotator 0.0 0.0 _returnvalue_7) false false)
  (AI|Components|Blackboard|SetValueasBool (AI|GetBlackboard 0) (Utilities|Name|MakeLiteralName "IsHeadMoving") _returnvalue_12)
  (if _returnvalue_12
    (Utilities|Time|ClearandInvalidateTimerbyHandle (Variables|Default|GetTurretHandle))))

(fn RotatetoDestination
  (bind _returnvalue (Actor|GetActorOfClass "/Game/NewSkye/Blueprint/BP_Destination.BP_Destination_C"))
  (Transformation|SetActorRotation (Math|Interpolation|RInterpTo (Transformation|GetActorRotation) (Math|Rotator|CombineRotators (Math|Rotator|MakeRotator 0.0 0.0 (* (Variables|Default|GetTargetTurnSpeed) (Utilities|Time|GetWorldDeltaSeconds))) (Math|Rotator|FindLookatRotation (Transformation|GetActorLocation) (Transformation|GetActorLocation _returnvalue))) (Utilities|Time|GetWorldDeltaSeconds) 3.0)))

(fn DistanceCalculate
  (bind _returnvalue (AI|GetBlackboard 0))
  (bind _returnvalue_2 (Utilities|Name|MakeLiteralName "RandomRot"))
  (bind _box1 (Variables|Default|GetBox1))
  (bind _returnvalue_3 (Class|BlackboardComponent|GetValueasRotator _returnvalue _returnvalue_2))
  (bind _relativerotation (Variables|/Script/Engine.SceneComponent|GetRelativeRotation _box1))
  (bind _returnvalue_4 (Math|Rotator|NormalizeAxis (.yaw _returnvalue_3)))
  (bind _returnvalue_5 (Math|Rotator|NormalizeAxis (.yaw _relativerotation)))
  (bind _returnvalue_6 (- _returnvalue_4 _returnvalue_5))
  (bind _returnvalue_7 (Math|Rotator|NormalizeAxis _returnvalue_6))
  (bind _returnvalue_8 (Math|Float|Absolute(Float) _returnvalue_7))
  (bind _returnvalue_9 (<= _returnvalue_8 5.0))
  (bind _returnvalue_10 (not _returnvalue_9))
  (Transformation|SetRelativeRotation (Variables|Default|GetBox1) (Math|Rotator|MakeRotator 0.0 0.0 (.yaw (Math|Interpolation|RInterpTo (Variables|/Script/Engine.SceneComponent|GetRelativeRotation (Variables|Default|GetBox1)) (Class|BlackboardComponent|GetValueasRotator (AI|GetBlackboard 0) (Utilities|Name|MakeLiteralName "RandomRot")) (Utilities|Time|GetWorldDeltaSeconds) 8.0))) false false)
  (AI|Components|Blackboard|SetValueasBool (AI|GetBlackboard 0) (Utilities|Name|MakeLiteralName "IsHeadMoving") _returnvalue_10)
  (if (not _returnvalue_10)
    (Utilities|Time|ClearandInvalidateTimerbyHandle (Variables|Default|GetRandomrotHandle))))

(fn GetMaxHealth
  (return (Variables|/Game/NewSkye/Blueprint/AI_DamageSystem/BPC_DamageSystem.BPC_DamageSystem_C|GetMaxHealth (Variables|Default|GetBPC_DamageSystem))))

(fn TakeDamage
  (params (DamageInfo :type My%20Damage%20Structure%20Structure))
  (bind _bpc_damagesystem (Variables|Default|GetBPC_DamageSystem))
  (|CallParentFunction DamageInfo)
  (bind _wasdamaged (Default|TakeDamage (Variables|Default|GetBPC_DamageSystem) DamageInfo))
  (if (Utilities|IsValid self)
    (bind _aswbp_health_bar (Utilities|Casting|CastToWBP_HealthBar (UserInterface|GetWidget (Variables|Default|GetHealthBar))))
    (Default|PercentUpdate _aswbp_health_bar (Variables|/Game/NewSkye/Blueprint/AI_DamageSystem/BPC_DamageSystem.BPC_DamageSystem_C|GetMaxHealth _bpc_damagesystem) (Variables|/Game/NewSkye/Blueprint/AI_DamageSystem/BPC_DamageSystem.BPC_DamageSystem_C|GetHealth _bpc_damagesystem))
    (return _wasdamaged)))

(fn GetCurrentHealth
  (return (Variables|/Game/NewSkye/Blueprint/AI_DamageSystem/BPC_DamageSystem.BPC_DamageSystem_C|GetHealth (Variables|Default|GetBPC_DamageSystem))))

(fn IsDead
  (return false))

(fn AlignHeadPivot
  (bind _returnvalue (Game|GetPlayerController 0))
  (bind _scene (Variables|Default|GetScene))
  (bind _returnvalue_2 (Transformation|GetWorldTransform _scene))
  (bind _returnvalue_3 (Pawn|GetControlledPawn _returnvalue))
  (bind _returnvalue_4 (Transformation|GetActorLocation _returnvalue_3))
  (bind _returnvalue_5 (Math|Transform|InverseTransformLocation _returnvalue_2 _returnvalue_4))
  (Transformation|SetRelativeRotation (Variables|Default|GetBox1) (Math|Rotator|MakeRotator 0.0 0.0 (Class|KismetMathLibrary|DegAtan2 (.y _returnvalue_5) (.x _returnvalue_5))) false false))

(fn GunRotatetoTargetActor
  (bind _returnvalue (Game|GetPlayerController 0))
  (bind _box1 (Variables|Default|GetBox1))
  (bind _box2 (Variables|Default|GetBox2))
  (bind _box2_2 (Variables|Default|GetBox2))
  (bind _box1_2 (Variables|Default|GetBox1))
  (bind _returnvalue_2 (Transformation|GetWorldTransform _box1))
  (bind _returnvalue_3 (Transformation|GetWorldLocation _box2))
  (bind _returnvalue_4 (Pawn|GetControlledPawn _returnvalue))
  (bind _returnvalue_5 (Transformation|GetWorldTransform _box1_2))
  (bind _relativerotation (Variables|/Script/Engine.SceneComponent|GetRelativeRotation _box2_2))
  (bind _returnvalue_6 (Transformation|GetActorLocation _returnvalue_4))
  (bind _returnvalue_7 (Math|Transform|InverseTransformLocation _returnvalue_2 _returnvalue_3))
  (bind _returnvalue_8 (- 0.0 (.roll _relativerotation)))
  (bind _returnvalue_9 (Math|Transform|InverseTransformLocation _returnvalue_5 _returnvalue_6))
  (bind _returnvalue_10 (Math|Rotator|NormalizeAxis _returnvalue_8))
  (bind _returnvalue_11 (Math|Float|Absolute(Float) _returnvalue_10))
  (bind _returnvalue_12 (- _returnvalue_9 _returnvalue_7))
  (bind _returnvalue_13 (<= _returnvalue_11 1.0))
  (bind _returnvalue_14 (not _returnvalue_13))
  (Transformation|SetRelativeRotation (Variables|Default|GetBox2) (Math|Rotator|MakeRotator 0.0 (Class|KismetMathLibrary|DegAtan2 (.z _returnvalue_12) (Math|Vector2D|Vector2DLength (Math|Vector2D|MakeVector2D (.x _returnvalue_12) (.y _returnvalue_12)))) 0.0) false false)
  (AI|Components|Blackboard|SetValueasBool (AI|GetBlackboard 0) (Utilities|Name|MakeLiteralName "IsGunMoving") _returnvalue_14)
  (if _returnvalue_14
    (Utilities|Time|ClearandInvalidateTimerbyHandle (Variables|Default|GetGunHandle))))