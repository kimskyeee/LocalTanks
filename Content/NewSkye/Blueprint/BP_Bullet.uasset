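; BP_Bullet is an enemy projectile actor that delivers shell damage to whatever it overlaps.
; On BeginPlay it loads the Pzgr41 shell data from ShellLibrary, applies the enemy missile collision preset and calls Active.
; On collision overlap it sends that shell data, its location and its reversed forward vector as impact normal through TakeDamageMessage, then destroys itself.
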(event OnComponentBeginOverlap(Collision)
  (params (OverlappedComponent :type Primitive%20Component%20Object%20Reference) (OtherActor :type Actor%20Object%20Reference) (OtherComp :type Primitive%20Component%20Object%20Reference) (OtherBodyIndex :type Integer) (bFromSweep :type Boolean) (SweepResult :type Hit%20Result%20Structure%20%28by%20ref%29))
  (Class|DamageInterface|TakeDamage(Message) OtherActor (Utilities|Struct|MakeMyDamageStructure (Variables|Default|GetShellInfo) (Transformation|GetActorLocation) false (* (Transformation|GetActorForwardVector) -1.0) 0.0))
  (Actor|DestroyActor))

(event EventTick
  (params (DeltaSeconds :type Float%20%28single-precision%29)))

(event EventBeginPlay
  (bind _returnvalue (Class|ShellLibrary|GetShellBasicInfo (Variables|Default|GetShellLibrary) "Pzgr41"))
  (Variables|Default|SetShellInfo _returnvalue)
  (Class|Shell|SetCollisionPreset "Enemy_Missile")
  (Class|Shell|Active))

(fn ConstructionScript)