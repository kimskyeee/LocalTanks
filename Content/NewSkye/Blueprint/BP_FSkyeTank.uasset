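; BP_FSkyeTank is a tank actor that drives over terrain, following its height and slope.
; Each tick it sums hit normals and heights from all BP_GroundSensing components and divides by the grounded count.
; The averaged normal and target turn speed drive an interpolated rotation.
; Movement is an unswept world offset combining smoothed forward speed with a height correction along the actor's up vector.
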(event EventBeginPlay
  (Variables|Default|SetGround%20Sensing (Actor|GetComponentsByClass "/Game/NewSkye/Blueprint/BP_GroundSensing.BP_GroundSensing_C")))

(event EventTick
  (params (DeltaSeconds :type Float%20%28single-precision%29))
  (bind _returnvalue (Utilities|Time|GetWorldDeltaSeconds))
  (bind _returnvalue_2 (Utilities|Time|GetWorldDeltaSeconds))
  (Variables|Default|SetAverageNormal "0, 0, 0")
  (Variables|Default|SetAverageHeight 0.0)
  (Variables|Default|SetCountOnGround 0)
  (for _array_element (Variables|Default|GetGround%20Sensing)
    (Variables|Default|SetAverageNormal (+ (Variables|/Game/NewSkye/Blueprint/BP_GroundSensing.BP_GroundSensing_C|GetHitNormal _array_element) (Variables|Default|GetAverageNormal)))
    (Variables|Default|SetAverageHeight (+ (.z (Variables|/Game/NewSkye/Blueprint/BP_GroundSensing.BP_GroundSensing_C|GetHitLocation _array_element)) (Variables|Default|GetAverageHeight)))
    (if (Variables|/Game/NewSkye/Blueprint/BP_GroundSensing.BP_GroundSensing_C|GetbOnGround _array_element)
      (Math|Integer|IncrementInt (Variables|Default|GetCountOnGround))))
  (Variables|Default|SetAverageNormal (/ (Variables|Default|GetAverageNormal) (Variables|Default|GetCountOnGround)))
  (bind _output_get (Variables|Default|SetAverageHeight (/ (Variables|Default|GetAverageHeight) (Variables|Default|GetCountOnGround))))
  (Variables|Default|SetDeltaZ (- (+ _output_get (Variables|Default|GetHeightOffset)) (.z (Transformation|GetActorLocation))))
  (Transformation|SetActorRotation (Math|Interpolation|RInterpTo (Transformation|GetActorRotation) (Math|Rotator|CombineRotators (Math|Rotator|MakeRotator 0.0 0.0 (* (Variables|Default|GetTargetTurnSpeed) _returnvalue_2)) (Math|Rotator|MakeRotfromZY (Variables|Default|GetAverageNormal) (Transformation|GetActorRightVector))) _returnvalue_2 8.0))
  (Transformation|AddActorWorldOffset (+ (* (Transformation|GetActorForwardVector) (Math|Interpolation|FInterpTo (Variables|Default|GetCurrentForwardSpeed) (Variables|Default|GetTargetForwardSpeed) _returnvalue 3.0) _returnvalue) (* (Transformation|GetActorUpVector) (Variables|Default|GetDeltaZ))))
  (Variables|Default|SetCurrentForwardSpeed (Math|Interpolation|FInterpTo (Variables|Default|GetCurrentForwardSpeed) (Variables|Default|GetTargetForwardSpeed) _returnvalue 3.0)))

(fn ConstructionScript)