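; Player-drivable T-72 tank pawn with Enhanced Input driving, turning, aiming and projectile firing from the Fire component.
; Each tick, averaged BP_GroundSensing normals tilt the mesh to terrain, while interpolated yaw and unswept world offsets move it.
; Look input rotates the spring arm and feeds turret and gun rotation to the AnimBP; hull turning counter-rotates the turret.
; BPC damage component handles health; death and block events only print.
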(event Custom|OnDeath
  (Development|PrintString "death"))

(event Custom|OnBlocked
  (params (blocked :type Boolean))
  (Development|PrintString "blocked"))

(event Input|EnhancedActionEvents|EnhancedInputActionIA_Fire
  (params (ActionValue :type Boolean) (ElapsedSeconds :type Float%20%28double-precision%29) (TriggeredSeconds :type Float%20%28double-precision%29) (InputAction :type Input%20Action%20Object%20Reference :default "/Game/MkTank/Input/IA_Fire.IA_Fire"))
  (:Started
    (Game|SpawnActorfromClass "/Game/MkTank/BluePrint/Bp_ProJectile.Bp_ProJectile_C" (Transformation|GetWorldTransform (Variables|Default|GetFire)) "AdjustIfPossibleButAlwaysSpawn" "MultiplyWithRoot" 0 0)))

(event Input|EnhancedActionEvents|EnhancedInputActionIA_Drive
  (params (ActionValue :type Float%20%28double-precision%29) (ElapsedSeconds :type Float%20%28double-precision%29) (TriggeredSeconds :type Float%20%28double-precision%29) (InputAction :type Input%20Action%20Object%20Reference :default "/Game/MkTank/Input/IA_Drive.IA_Drive"))
  (:Triggered
    (Variables|Default|SetDrive%20Speed (+ ActionValue (Variables|Default|GetDrive%20Speed))))
  (:Completed
    (Variables|Default|SetDrive%20Speed 0.0)))

(event Input|EnhancedActionEvents|EnhancedInputActionIA_TurnAD
  (params (ActionValue :type Float%20%28double-precision%29) (ElapsedSeconds :type Float%20%28double-precision%29) (TriggeredSeconds :type Float%20%28double-precision%29) (InputAction :type Input%20Action%20Object%20Reference :default "/Game/MkTank/Input/IA_TurnAD.IA_TurnAD"))
  (bind _as_abp_east_tank_t72b (Variables|Default|GetAs%20ABP%20East%20Tank%20T72b))
  (:Triggered
    (Variables|Default|SetTurn%20Speed (+ ActionValue (Variables|Default|GetTurn%20Speed)))
    (Variables|/Game/VigilanteContent/Vehicles/East_Tank_T72b/ABP_East_Tank_T72b.ABP_East_Tank_T72b_C|SetTurretRotation _as_abp_east_tank_t72b (Math|Rotator|MakeRotator (.roll (Variables|/Game/VigilanteContent/Vehicles/East_Tank_T72b/ABP_East_Tank_T72b.ABP_East_Tank_T72b_C|GetTurretRotation _as_abp_east_tank_t72b)) (.pitch (Variables|/Game/VigilanteContent/Vehicles/East_Tank_T72b/ABP_East_Tank_T72b.ABP_East_Tank_T72b_C|GetTurretRotation _as_abp_east_tank_t72b)) (Math|Interpolation|FInterpTo (.yaw (Variables|/Game/VigilanteContent/Vehicles/East_Tank_T72b/ABP_East_Tank_T72b.ABP_East_Tank_T72b_C|GetTurretRotation _as_abp_east_tank_t72b)) (- (.yaw (Variables|/Game/VigilanteContent/Vehicles/East_Tank_T72b/ABP_East_Tank_T72b.ABP_East_Tank_T72b_C|GetTurretRotation _as_abp_east_tank_t72b)) (Variables|Default|GetTurn%20Speed)) (Utilities|Time|GetWorldDeltaSeconds) 2.0))))
  (:Completed
    (Variables|Default|SetTurn%20Speed 0.0)))

(event Input|EnhancedActionEvents|EnhancedInputActionIA_LookTurn
  (params (ActionValue :type Float%20%28double-precision%29) (ElapsedSeconds :type Float%20%28double-precision%29) (TriggeredSeconds :type Float%20%28double-precision%29) (InputAction :type Input%20Action%20Object%20Reference :default "/Game/MkTank/Input/IA_LookTurn.IA_LookTurn"))
  (bind _as_abp_east_tank_t72b (Variables|Default|GetAs%20ABP%20East%20Tank%20T72b))
  (bind _springarm (Variables|Default|GetSpringArm))
  (bind _returnvalue (Transformation|GetWorldRotation _springarm))
  (Transformation|SetWorldRotation _springarm (Math|Rotator|MakeRotator 0.0 (+ (- 0.0 (stale Input|EnhancedActionEvents|EnhancedInputActionIA_LookUp ActionValue)) (.pitch _returnvalue)) (+ (.yaw _returnvalue) ActionValue)) false false)
  (Variables|/Game/VigilanteContent/Vehicles/East_Tank_T72b/ABP_East_Tank_T72b.ABP_East_Tank_T72b_C|SetTurretRotation _as_abp_east_tank_t72b (Math|Rotator|MakeRotator 0.0 0.0 (Math|Interpolation|FInterpTo (.yaw (Variables|/Game/VigilanteContent/Vehicles/East_Tank_T72b/ABP_East_Tank_T72b.ABP_East_Tank_T72b_C|GetTurretRotation _as_abp_east_tank_t72b)) (+ ActionValue (.yaw (Variables|/Game/VigilanteContent/Vehicles/East_Tank_T72b/ABP_East_Tank_T72b.ABP_East_Tank_T72b_C|GetTurretRotation _as_abp_east_tank_t72b))) 0.2 4.0)))
  (bind _output_get (Variables|Default|SetGun%20Rot (+ (Variables|Default|GetGun%20Rot) (- 0.0 (stale Input|EnhancedActionEvents|EnhancedInputActionIA_LookUp ActionValue)))))
  (Variables|/Game/VigilanteContent/Vehicles/East_Tank_T72b/ABP_East_Tank_T72b.ABP_East_Tank_T72b_C|SetGunRotation _as_abp_east_tank_t72b (Math|Rotator|MakeRotator 0.0 (Math|Float|Clamp(Float) _output_get -45.0 9e+01) 0.0)))

(event Input|EnhancedActionEvents|EnhancedInputActionIA_LookUp
  (params (ActionValue :type Float%20%28double-precision%29) (ElapsedSeconds :type Float%20%28double-precision%29) (TriggeredSeconds :type Float%20%28double-precision%29) (InputAction :type Input%20Action%20Object%20Reference :default "/Game/MkTank/Input/IA_LookUp.IA_LookUp"))
  (bind _as_abp_east_tank_t72b (Variables|Default|GetAs%20ABP%20East%20Tank%20T72b))
  (bind _springarm (Variables|Default|GetSpringArm))
  (bind _returnvalue (Transformation|GetWorldRotation _springarm))
  (Transformation|SetWorldRotation _springarm (Math|Rotator|MakeRotator 0.0 (+ (- 0.0 ActionValue) (.pitch _returnvalue)) (+ (.yaw _returnvalue) (stale Input|EnhancedActionEvents|EnhancedInputActionIA_LookTurn ActionValue))) false false)
  (Variables|/Game/VigilanteContent/Vehicles/East_Tank_T72b/ABP_East_Tank_T72b.ABP_East_Tank_T72b_C|SetTurretRotation _as_abp_east_tank_t72b (Math|Rotator|MakeRotator 0.0 0.0 (Math|Interpolation|FInterpTo (.yaw (Variables|/Game/VigilanteContent/Vehicles/East_Tank_T72b/ABP_East_Tank_T72b.ABP_East_Tank_T72b_C|GetTurretRotation _as_abp_east_tank_t72b)) (+ (stale Input|EnhancedActionEvents|EnhancedInputActionIA_LookTurn ActionValue) (.yaw (Variables|/Game/VigilanteContent/Vehicles/East_Tank_T72b/ABP_East_Tank_T72b.ABP_East_Tank_T72b_C|GetTurretRotation _as_abp_east_tank_t72b))) 0.2 4.0)))
  (bind _output_get (Variables|Default|SetGun%20Rot (+ (Variables|Default|GetGun%20Rot) (- 0.0 ActionValue))))
  (Variables|/Game/VigilanteContent/Vehicles/East_Tank_T72b/ABP_East_Tank_T72b.ABP_East_Tank_T72b_C|SetGunRotation _as_abp_east_tank_t72b (Math|Rotator|MakeRotator 0.0 (Math|Float|Clamp(Float) _output_get -45.0 9e+01) 0.0)))

(event EventBeginPlay
  (bind _springarm (Variables|Default|GetSpringArm))
  (Input|AddMappingContext (PlayerController|LocalPlayerSubsystems|GetEnhancedInputLocalPlayerSubsystem (Game|GetPlayerController 0)) "/Game/MkTank/Input/IMC_Tank.IMC_Tank" 0 "(bIgnoreAllPressedKeysUntilRelease=True,bForceImmediately=False,bNotifyUserSettings=False)")
  (Variables|Default|SetGroundSensingArray (Actor|GetComponentsByClass "/Game/MkTank/BluePrint/BP_GroundSensing.BP_GroundSensing_C"))
  (bind _asabp_east_tank_t72b (Utilities|Casting|CastToABP_East_Tank_T72b (Components|SkeletalMesh|GetAnimInstance (Variables|Default|GetSkeletalMesh))))
  (Variables|Default|SetAs%20ABP%20East%20Tank%20T72b _asabp_east_tank_t72b)
  (Transformation|SetWorldRotation _springarm (Math|Rotator|MakeRotator 0.0 (+ (.pitch (Class|SpringArmComponent|GetTargetRotation _springarm)) -1e+01) 0.0) false false))

(event EventTick
  (params (DeltaSeconds :type Float%20%28single-precision%29))
  (bind _returnvalue (Utilities|Time|GetWorldDeltaSeconds))
  (bind _skeletalmesh (Variables|Default|GetSkeletalMesh))
  (bind _fire (Variables|Default|GetFire))
  (bind _returnvalue_2 (Transformation|GetWorldLocation _fire))
  (bind _returnvalue_3 (Transformation|GetWorldRotation _skeletalmesh))
  (bind _returnvalue_4 (Transformation|GetWorldRotation _skeletalmesh))
  (bind _outhit (Collision|LineTraceByChannel _returnvalue_2 (+ _returnvalue_2 (* (Math|Vector|GetForwardVector _fire) (Variables|Default|GetDistance))) "TraceTypeQuery1" false 0 "ForOneFrame"))
  (Variables|Default|SetAverageNormal "0, 0, 0")
  (Variables|Default|SetAvereageHeight 0.0)
  (Variables|Default|SetCountOnGround 0)
  (for _array_element (Variables|Default|GetGroundSensingArray)
    (Variables|Default|SetAverageNormal (+ (Variables|/Game/MkTank/BluePrint/BP_GroundSensing.BP_GroundSensing_C|GetHitNormal _array_element) (Variables|Default|GetAverageNormal)))
    (Variables|Default|SetAvereageHeight (+ (.z (Variables|/Game/MkTank/BluePrint/BP_GroundSensing.BP_GroundSensing_C|GetHitNormal _array_element)) (Variables|Default|GetAvereageHeight)))
    (Variables|Default|SetAva%20Hit%20Location (+ (Variables|/Game/MkTank/BluePrint/BP_GroundSensing.BP_GroundSensing_C|GetHitLocation _array_element) (Variables|Default|GetAva%20Hit%20Location)))
    (if (Variables|/Game/MkTank/BluePrint/BP_GroundSensing.BP_GroundSensing_C|GetbOnGround _array_element)
      (Math|Integer|IncrementInt (Variables|Default|GetCountOnGround))))
  (Variables|Default|SetAverageNormal (/ (Variables|Default|GetAverageNormal) (Variables|Default|GetCountOnGround)))
  (bind _output_get (Variables|Default|SetAvereageHeight (/ (Variables|Default|GetAvereageHeight) (Variables|Default|GetCountOnGround))))
  (Variables|Default|SetDeltaZ (- (+ _output_get (Variables|Default|GetHeightOffset)) (.z (Transformation|GetActorLocation))))
  (Transformation|SetWorldRotation _skeletalmesh (Math|Rotator|MakeRotator (Math|Interpolation|FInterpTo (.roll _returnvalue_4) (.roll (Math|Rotator|MakeRotfromZY (Variables|Default|GetAverageNormal) (Math|Vector|GetRightVector _skeletalmesh))) _returnvalue 8.0) (Math|Interpolation|FInterpTo (.pitch _returnvalue_4) (.pitch (Math|Rotator|MakeRotfromZY (Variables|Default|GetAverageNormal) (Math|Vector|GetRightVector _skeletalmesh))) _returnvalue 8.0) (Math|Interpolation|FInterpTo (.yaw _returnvalue_3) (+ (.yaw _returnvalue_3) (Variables|Default|GetTurn%20Speed)) (Utilities|Time|GetWorldDeltaSeconds) 2.0)) false false)
  (Transformation|AddActorWorldOffset (* (Math|Interpolation|FInterpTo (Variables|Default|GetCurrentForwardSpeed) (Variables|Default|GetDrive%20Speed) 0.1 32.0) (Math|Vector|GetForwardVector (Variables|Default|GetSkeletalMesh)) (Utilities|Time|GetWorldDeltaSeconds))))

(fn ConstructionScript
  (bind _bpc_damagesystem (Variables|Default|GetBPC_DamageSystem))
  (EventDispatchers|BindEventtoOnDeath _bpc_damagesystem (EventDispatchers|CreateEvent :!event Custom|OnDeath))
  (EventDispatchers|BindEventtoOnBlocked _bpc_damagesystem (EventDispatchers|CreateEvent :!event Custom|OnBlocked)))

(fn TakeDamage
  (params (DamageInfo :type My%20Damage%20Structure%20Structure))
  (bind _returnvalue (Class|DamageInterface|TakeDamage(Message) (Variables|Default|GetBPC_DamageSystem) DamageInfo))
  (return _returnvalue))

(fn GetMaxHealth
  (return (Variables|/Game/NewSkye/Blueprint/AI_DamageSystem/BPC_DamageSystem.BPC_DamageSystem_C|GetMaxHealth (Variables|Default|GetBPC_DamageSystem))))

(fn GetCurrentHealth
  (return (Variables|/Game/NewSkye/Blueprint/AI_DamageSystem/BPC_DamageSystem.BPC_DamageSystem_C|GetHealth (Variables|Default|GetBPC_DamageSystem))))