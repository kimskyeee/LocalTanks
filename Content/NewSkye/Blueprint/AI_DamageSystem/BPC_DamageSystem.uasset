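; BPC_DamageSystem is a Blueprint component that tracks health and death for its owning actor.
; Health resets to MaxHealth on BeginPlay.
; TakeDamage subtracts the shell damage from the incoming damage info, and when health reaches zero or below it sets IsDead and fires the OnDeath dispatcher.
; It always returns true and has no guard against further hits after death.
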(event EventBeginPlay
  (Variables|Default|SetHealth (Variables|Default|GetMaxHealth)))

(event EventTick
  (params (DeltaSeconds :type Float%20%28single-precision%29)))

(fn TakeDamage
  (params (DamageInfo :type My%20Damage%20Structure%20Structure))
  (bind _output_get (Variables|Default|SetHealth (- (Variables|Default|GetHealth) (.ShellDamage (Utilities|Struct|BreakShellBasicInfo (.ShellBasicInfo (Utilities|Struct|BreakMyDamageStructure DamageInfo)))))))
  (if (<= _output_get 0.0)
    (Variables|Default|SetIsDead true)
    (Default|CallOnDeath))
  (return true))